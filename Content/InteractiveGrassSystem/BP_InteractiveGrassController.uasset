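; Controller for interactive grass that renders vector field emitter proxies through a top-down orthographic scene capture over a configurable world area.
; The construction script sizes the capture, bounds and clear quad from WorldSize and WorldHeight.
; BeginPlay enables the effect and publishes capture center and half-size through MPC_InteractiveGrass.
; CreateProxy attaches sphere emitters to targets; AttachProxy adds them to the capture's show-only list and hides them from the player.
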(event `self.ReceiveBeginPlay`
  (bind _capturecomponent2d (`self.CaptureComponent2D`))
  (bind _returnvalue (* (`self.WorldSize`) 0.5))
  (`KismetMaterialLibrary.SetVectorParameterValue` "/Game/InteractiveGrassSystem/MPC_InteractiveGrass.MPC_InteractiveGrass" "WorldCenterAndHalfSize" (make `LinearColor` (.x (`SceneComponent.K2_GetComponentLocation` (`self.CaptureComponent2D`))) (.y (`SceneComponent.K2_GetComponentLocation` (`self.CaptureComponent2D`))) _returnvalue _returnvalue))
  (`SceneComponent.K2_SetWorldRotation` _capturecomponent2d (struct :`Pitch` -90.0 :`Yaw` -90.0) false true)
  (`SceneCaptureComponent.ShowOnlyComponent` _capturecomponent2d (`self.ClearQuad`))
  (`KismetMaterialLibrary.SetScalarParameterValue` "/Game/InteractiveGrassSystem/MPC_InteractiveGrass.MPC_InteractiveGrass" "EnableInteractiveGrass" 1.0)
  (set `SceneCaptureComponent2D.ProjectionType` "Orthographic" _capturecomponent2d))

(fn `AttachProxy`
  (params (ProxyActor :type "Actor Object Reference"))
  (`SceneCaptureComponent.ShowOnlyActorComponents` (`self.CaptureComponent2D`) ProxyActor)
  (`KismetRenderingLibrary.HideActor` (`GameplayStatics.GetPlayerController` 0) ProxyActor))

(fn `CreateProxy`
  (params (Target :type "SceneComponent Object Reference"))
  (bind _returnvalue (`|SpawnActorFromClass` "/Game/InteractiveGrassSystem/BP_SphereVectorFieldEmitterActor.BP_SphereVectorFieldEmitterActor_C" (`SceneComponent.K2_GetComponentToWorld` Target) "Undefined" "OverrideRootScale" (`ActorComponent.GetOwner` (`self.CaptureComponent2D`)) null))
  (`self.K2_AttachToComponent` _returnvalue Target "None" "SnapToTarget" "SnapToTarget" "SnapToTarget" true)
  (`self.AttachProxy` _returnvalue))

(fn `RemoveProxy`
  (params (Target :type "SceneComponent Object Reference"))
  (`BlueprintMapLibrary.Map_Remove` (`self._GrassProxy`) Target))

(fn `UserConstructionScript`
  (bind _worldsize (`self.WorldSize`))
  (bind _capturecomponent2d (`self.CaptureComponent2D`))
  (bind _returnvalue (* _worldsize 0.5))
  (bind _returnvalue_2 (* (`self.WorldSize`) 0.5))
  (`BoxComponent.SetBoxExtent` (`self.WorldBound`) (`KismetMathLibrary.MakeVector` (`self.WorldHeight`) _returnvalue _returnvalue) false)
  (set `SceneCaptureComponent2D.OrthoWidth` _worldsize _capturecomponent2d)
  (`SceneComponent.K2_AddWorldOffset` (`self.WorldBound`) (`KismetMathLibrary.MakeVector` 0.0 0.0 (* (`self.WorldHeight`) -1.0)) false false)
  (`SceneComponent.K2_AddWorldOffset` (`self.ClearQuad`) (`KismetMathLibrary.MakeVector` 0.0 0.0 (* (`self.WorldHeight`) -2.0)) false false)
  (`SceneComponent.SetWorldScale3D` (`self.ClearQuad`) (`KismetMathLibrary.Conv_DoubleToVector` (* (`self.WorldSize`) 0.01)))
  (`SceneComponent.K2_SetWorldRotation` (`Actor.RootComponent` (`ActorComponent.GetOwner` _capturecomponent2d)) (struct :`Pitch` -90.0 :`Yaw` -90.0) false false)
  (`KismetMaterialLibrary.SetVectorParameterValue` null "WorldCenterAndHalfSize" (make `LinearColor` (.x (`SceneComponent.K2_GetComponentLocation` _capturecomponent2d)) (.y (`SceneComponent.K2_GetComponentLocation` _capturecomponent2d)) _returnvalue_2 _returnvalue_2))
  (set `SceneCaptureComponent2D.ProjectionType` "Orthographic" (`self.CaptureComponent2D`)))