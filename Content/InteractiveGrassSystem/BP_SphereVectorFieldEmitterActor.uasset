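; Sphere vector field emitter actor for the interactive grass system, wrapping a particle system.
; The construction script picks a complex, static or movable particle template from VectorFieldType and sizes it uniformly through the FieldSize parameter.
; On BeginPlay it attaches itself as a proxy to the first BP_InteractiveGrassController found.
; A fixed world rotation is reapplied every tick, and Reset restarts the particle system.
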(event `self.ReceiveBeginPlay`
  (bind _outactors (`GameplayStatics.GetAllActorsOfClass` "/Game/InteractiveGrassSystem/BP_InteractiveGrassController.BP_InteractiveGrassController_C"))
  (`/Game/InteractiveGrassSystem/BP_InteractiveGrassController.AttachProxy` (`|GetArrayItem` _outactors) (`ActorComponent.GetOwner` (`self.ParticleSystem`))))

(event `self.ReceiveTick`
  (params (DeltaSeconds :type "Float (single-precision)"))
  (`SceneComponent.K2_SetWorldRotation` (`self.ParticleSystem`) (struct :`Yaw` -45.0) false false))

(fn `Reset`
  (bind _particlesystem (`self.ParticleSystem`))
  (`ActorComponent.SetActive` _particlesystem false true)
  (`ActorComponent.SetActive` _particlesystem true true))

(fn `UserConstructionScript`
  (bind _vectorfieldsize (`self.VectorFieldSize`))
  (bind _particlesystem (`self.ParticleSystem`))
  (switch `/Game/InteractiveGrassSystem/BP_InteractiveGrassVectorFieldType` (`self.VectorFieldType`)
    (:`NewEnumerator0`
      (`ParticleSystemComponent.SetTemplate` _particlesystem (`self.ComplexTemplate`)))
    (:`NewEnumerator1`
      (`ParticleSystemComponent.SetTemplate` _particlesystem (`self.StaticTemplate`)))
    (:`NewEnumerator2`
      (`ParticleSystemComponent.SetTemplate` _particlesystem (`self.MovableTemplate`))))
  (`ParticleSystemComponent.SetVectorParameter` (`self.ParticleSystem`) "FieldSize" (`KismetMathLibrary.MakeVector` _vectorfieldsize _vectorfieldsize _vectorfieldsize))
  (`SceneComponent.K2_SetWorldRotation` (`self.ParticleSystem`) (struct :`Yaw` -45.0) false false))